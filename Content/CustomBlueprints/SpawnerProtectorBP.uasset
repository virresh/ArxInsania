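; Spawner and safe-zone actor that periodically drops damaging pumpkins around the player, except while the player is inside its protection box.
; A Delay on Tick paces spawns at randomly offset, raised locations near the player, capped by a count of DamagingBoulderBP actors rather than pumpkins.
; Overlap events toggle the character's NoSpawn flag and, when CanPray is set, a HUD prayer prompt.
; Pressing J inside a prayable box refreshes player stats.
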(event `self.ReceiveTick`
  (params (DeltaSeconds :type "Float (single-precision)"))
  ;[1 1 1] Perform Actual Spawning
  (`KismetSystemLibrary.Delay` (`self.SpawnDelay`))
  (bind _asfirst_person_character (cast `/Game/FirstPersonBP/Blueprints/FirstPersonCharacter` (`GameplayStatics.GetPlayerCharacter` 0)))
  (if (not (`/Game/FirstPersonBP/Blueprints/FirstPersonCharacter.NoSpawn` _asfirst_person_character))
    (bind _outactors (`GameplayStatics.GetAllActorsOfClass` "/Game/CustomBlueprints/DamagingBoulderBP.DamagingBoulderBP_C"))
    (if (< (`KismetArrayLibrary.Array_Length` _outactors) (`self.MaxBoulders`))
      (bind _location (.location (`self.GetTransform` _asfirst_person_character)))
      (`|SpawnActorFromClass` "/Game/CustomBlueprints/DamagingPumpkinBP.DamagingPumpkinBP_C" (`KismetMathLibrary.MakeTransform` (`KismetMathLibrary.MakeVector` (.x (+ _location (* (`KismetMathLibrary.RandomUnitVector`) 200))) (.y (+ _location (* (`KismetMathLibrary.RandomUnitVector`) 200))) (+ (.z _location) 100.0)) (`KismetMathLibrary.RandomRotator` true) (.scale (`self.GetTransform` _asfirst_person_character))) "AdjustIfPossibleButDontSpawnIfColliding" "OverrideRootScale" null null))))

(event `self.ReceiveBeginPlay`
  ;[1 1 1] Enable input for capturing J key
  (`self.EnableInput` (`GameplayStatics.GetPlayerController` 0)))

(event `self.ReceiveActorBeginOverlap`
  (params (OtherActor :type "Actor Object Reference"))
  ;[1 1 1] Don't spawn when inside protection box
  (bind _asfirst_person_character (cast `/Game/FirstPersonBP/Blueprints/FirstPersonCharacter` OtherActor))
  (set `/Game/FirstPersonBP/Blueprints/FirstPersonCharacter.NoSpawn` true _asfirst_person_character)
  (if (`self.CanPray?`)
    ;[1 1 1] Show praying option
    (`/Game/CustomBlueprints/HUD.RandomMessage` (`/Game/FirstPersonBP/Blueprints/FirstPersonCharacter.HUDRef` _asfirst_person_character) "Press J for Jai Shree Ram!")))

(event `self.ReceiveActorEndOverlap`
  (params (OtherActor :type "Actor Object Reference"))
  ;[1 1 1] Don't spawn when inside protection box
  (bind _asfirst_person_character (cast `/Game/FirstPersonBP/Blueprints/FirstPersonCharacter` OtherActor))
  (set `/Game/FirstPersonBP/Blueprints/FirstPersonCharacter.NoSpawn` false _asfirst_person_character)
  (if (`self.CanPray?`)
    ;[1 1 1] Hide Praying Option
    (`/Game/CustomBlueprints/HUD.RandomMessage` (`/Game/FirstPersonBP/Blueprints/FirstPersonCharacter.HUDRef` _asfirst_person_character) "")))

(event `Key|J` :consume false
  (params (Key :type "Key Structure"))
  ;[1 1 1] Handle logic for healing after praying
  (:`Pressed`
    (if (`self.CanPray?`)
      (bind _asfirst_person_character (cast `/Game/FirstPersonBP/Blueprints/FirstPersonCharacter` (`GameplayStatics.GetPlayerCharacter` 0)))
      (if (`self.IsOverlappingActor` _asfirst_person_character)
        (`/Game/FirstPersonBP/Blueprints/FirstPersonCharacter.Refresh Stats` _asfirst_person_character)))))

(fn `UserConstructionScript`)