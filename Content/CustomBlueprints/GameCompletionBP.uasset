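; GameCompletionBP is a trigger actor that completes a level once the player has collected enough Booti.
; On overlap with a FirstPersonCharacter whose NumBooti meets MinBooti, it shows the LevelCode message through that character's HUD and sets GameOver.
; It enables input on BeginPlay, and pressing C calls NextLevel on the player character, with no check of its own that the level is complete.
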(event `self.ReceiveBeginPlay`
  (`self.EnableInput` (`GameplayStatics.GetPlayerController` 0)))

(event `self.ReceiveActorBeginOverlap`
  (params (OtherActor :type "Actor Object Reference"))
  (bind _asfirst_person_character (cast `/Game/FirstPersonBP/Blueprints/FirstPersonCharacter` OtherActor))
  (if (>= (`/Game/FirstPersonBP/Blueprints/FirstPersonCharacter.NumBooti` _asfirst_person_character) (`self.MinBooti`))
    (`/Game/CustomBlueprints/HUD.DisplayLvlMsg` (`/Game/FirstPersonBP/Blueprints/FirstPersonCharacter.HUDRef` _asfirst_person_character) (`self.LevelCode`))
    (set `/Game/FirstPersonBP/Blueprints/FirstPersonCharacter.GameOver` true _asfirst_person_character)))

(event `Key|C`
  (params (Key :type "Key Structure"))
  (:`Pressed`
    (bind _asfirst_person_character (cast `/Game/FirstPersonBP/Blueprints/FirstPersonCharacter` (`GameplayStatics.GetPlayerCharacter` 0)))
    (`/Game/FirstPersonBP/Blueprints/FirstPersonCharacter.Next Level` _asfirst_person_character (`self.NextLevel`))))

(fn `UserConstructionScript`)