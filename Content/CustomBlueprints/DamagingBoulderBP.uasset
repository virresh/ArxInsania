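; DamagingBoulderBP is a short-lived boulder hazard that hurts players and can be broken by projectiles, destroying itself three seconds after spawning.
; Projectile hits on its Destructible component increment a counter until, from the third hit, it enables physics and applies radial damage.
; Hitting a FirstPersonCharacter calls its GetHitDamage, launches it along the hit normal with added lift, then jumps into that same break branch.
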(event `self.ReceiveBeginPlay`
  (`KismetSystemLibrary.Delay` 3.0)
  (`self.K2_DestroyActor`))

(event `self.Destructible.OnComponentHit`
  (params (HitComponent :type "PrimitiveComponent Object Reference") (OtherActor :type "Actor Object Reference") (OtherComp :type "PrimitiveComponent Object Reference") (NormalImpulse :type "Vector Structure") (Hit :type "HitResult Structure (by ref)"))
  (bind _asfirst_person_projectile (cast `/Game/FirstPersonBP/Blueprints/FirstPersonProjectile` OtherActor))
  (if (>= (`self.IsStacked5`) 2.0)
    (`PrimitiveComponent.SetSimulatePhysics` (`self.Destructible`) true :!label _label)
    (`GameplayStatics.ApplyRadialDamage` :`BaseDamage` 10.0 :`Origin` (`.ImpactPoint` (`GameplayStatics.BreakHitResult` Hit)) :`DamageRadius` 60.0 :`DamageTypeClass` "/Script/Engine.DamageType" :`DamageCauser` _asfirst_person_projectile :`InstigatedByController` null :`bDoFullDamage` true)
    (else
      (set `self.IsStacked5` (+ (`self.IsStacked5`) 1.0)))))

(event `self.ReceiveHit`
  (params (MyComp :type "PrimitiveComponent Object Reference") (Other :type "Actor Object Reference") (OtherComp :type "PrimitiveComponent Object Reference") (bSelfMoved :type Boolean) (HitLocation :type "Vector Structure") (HitNormal :type "Vector Structure") (NormalImpulse :type "Vector Structure") (Hit :type "HitResult Structure (by ref)"))
  (bind _asfirst_person_character (cast `/Game/FirstPersonBP/Blueprints/FirstPersonCharacter` Other))
  (`/Game/FirstPersonBP/Blueprints/FirstPersonCharacter.GetHitDamage` _asfirst_person_character)
  (`/Engine/EditorBlueprintResources/StandardMacros.IsValid` _asfirst_person_character
    (:`Is Valid`
      (`Character.LaunchCharacter` _asfirst_person_character (`KismetMathLibrary.MakeVector` (.x (* HitNormal 50)) (.y (* HitNormal 50)) (+ (.z (* HitNormal 50)) 100.0)) false false)
      (goto _label))))

(fn `UserConstructionScript`)